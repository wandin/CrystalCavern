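; BP_CollectableCrystal is a pickup crystal that animates into the player when touched, then destroys itself.
; On player overlap it caches its starting location, scale and light intensity, then plays a timeline.
; The timeline's separate tracks lerp it toward the player pawn's current position, shrink it to zero and fade its light out.
; It contains no score or inventory logic, only the collection effect.
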(event Collision|EventActorBeginOverlap
  (params (OtherActor :type Actor%20Object%20Reference))
  ;[1 1 1] Player collects the crystals - move crystals towards player, change its scale and luminosity
  (Utilities|IsPlayer OtherActor
    (:ISPlayer
      (CallFunction|StoreStartingValues)
      (bind (_direction _crystal_collection_progress _light_intensity _scale_progress) (Timeline|Crystal%20Colletion%20TImeline Play)
        (:Update
          (CallFunction|MovetoPlayer _crystal_collection_progress)
          (CallFunction|ScaleCrystal _scale_progress)
          (CallFunction|AdjustCrystalLuminosity _light_intensity))
        (:Finished
          (Actor|DestroyActor))))))

(fn ConstructionScript)

(fn MovetoPlayer
  (params (Alpha :type Float%20%28single-precision%29))
  (Transformation|SetActorLocation (Math|Vector|Lerp(Vector) (Variables|Default|GetStart%20Location) (Transformation|GetActorLocation (Game|Player|GetPlayerPawn 0)) Alpha) false false))

(fn StoreStartingValues
  (Variables|Default|SetStart%20Location (Transformation|GetActorLocation))
  (Variables|Default|SetStart%20Scale (Transformation|GetActorScale3D))
  (Variables|Default|SetStart%20Light%20Intensity (Variables|/Script/Engine.LightComponentBase|GetIntensity (Variables|Default|GetCrystal%20Light))))

(fn ScaleCrystal
  (params (Alpha :type Float%20%28single-precision%29))
  (Transformation|SetActorScale3D (Math|Vector|Lerp(Vector) (Variables|Default|GetStart%20Scale) "0, 0, 0" Alpha)))

(fn AdjustCrystalLuminosity
  (params (Alpha :type Float%20%28single-precision%29))
  (Rendering|Components|Light|SetIntensity (Variables|Default|GetCrystal%20Light) (Math|Float|Lerp (Variables|Default|GetStart%20Light%20Intensity) 0.0 Alpha)))