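; Level-end trigger actor that completes the level when the player overlaps it and no BP_CollectableCrystal actors remain.
; After a short delay, it finds the current level's name in the LevelNames array and opens the next entry by name.
; On the last entry, it prints a congratulations message and quits the game immediately, although the message announces a countdown.
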(event Collision|EventActorBeginOverlap
  (params (OtherActor :type Actor%20Object%20Reference))
  (Utilities|IsPlayer OtherActor
    (:ISPlayer
      (if (not (CallFunction|AnyCrystalsRemaining))
        (Utilities|FlowControl|Delay 5.0)
        (LevelManagement|CompleteLevel)))))

(fn ConstructionScript)

(fn AnyCrystalsRemaining
  (bind _outactors (Actor|GetAllActorsOfClass "/Game/Blueprints/Actors/Collectables/BP_CollectableCrystal.BP_CollectableCrystal_C"))
  (return (> (Utilities|Array|Length _outactors) 0)))

(fn CompleteLevel
  (if (LevelManagement|IsFinalLevel)
    (Development|PrintString "Congratulations!, You cleared both levels, the game will quit in 5 seconds" true true "(R=1.000000,G=0.921747,B=0.000000,A=1.000000)" 7.0)
    (Game|QuitGame 0 "Quit" false)
    (else
      (LevelManagement|LoadNextLevel))))

(fn IsFinalLevel
  (return (== (Utilities|Array|LastIndex (Variables|Default|GetLevelNames)) (LevelManagement|GetCurrentLevelIndex))))

(fn GetCurrentLevelIndex
  (bind _returnvalue (Game|GetCurrentLevelName true))
  (return (Utilities|Array|FindItem (Variables|Default|GetLevelNames) (Utilities|String|StringToName _returnvalue))))

(fn LoadNextLevel
  (Game|OpenLevel(byName) (LevelManagement|GetNextLevelName)))

(fn GetNextLevelName
  (return (Utilities|Array|Get(acopy) (Variables|Default|GetLevelNames) (+ (LevelManagement|GetCurrentLevelIndex) 1))))