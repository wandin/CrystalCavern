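; BP_Cannon is a cannon actor that fires automatically and repeatedly from BeginPlay.
; After a FireRate delay, it spawns a BP_Projectile at the arrow spawn point's location and rotation, scaled by ProjectileScale.
; A timeline then animates the barrel mesh along its relative Y axis, and the timeline's Cannon Fired output restarts the delay to close the firing loop.
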(event EventBeginPlay
  ;[1 1 1] Spawn - Firing Projectiles
  (Utilities|FlowControl|Delay (Variables|CannonFireProperties|GetFireRate) :!label _label)
  (CallFunction|FireProjectiles)
  ;[1 1 1] Cannon Barrel movement
  (bind _cannon_barrel_location (Timeline|Cannon%20FireMovement%20Timeline PlayFromStart)
    (:Update
      (CallFunction|MoveCannonBarrel _cannon_barrel_location))
    (:Cannon%20Fired
      (goto _label))))

(fn ConstructionScript)

(fn FireProjectiles
  (bind _arrow___projectile_spawn_point (Variables|Default|GetArrow%20-%20Projectile%20Spawn%20Point))
  (Game|SpawnActorfromClass "/Game/Blueprints/Actors/Projectiles/BP_Projectile.BP_Projectile_C" (Math|Transform|MakeTransform (Transformation|GetWorldLocation _arrow___projectile_spawn_point) (Transformation|GetWorldRotation _arrow___projectile_spawn_point) (Math|Conversions|ToVector(Float) (Variables|CannonFireProperties|GetProjectileScale))) "Undefined" 0 0))

(fn MoveCannonBarrel
  (params (CannonBarrelYLocation :type Float%20%28single-precision%29))
  (Transformation|SetRelativeLocation (Variables|Default|GetStaticMesh%20-%20Cannon%20barrel) (Math|Vector|MakeVector 0.0 CannonBarrelYLocation 0.0) false false))